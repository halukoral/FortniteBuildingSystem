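; BP_BuildingManager is the building system manager that sets up construction UI and selection for the player.
; On init it casts the player character, caches it, and asks the player's main widget to generate building widgets, which it stores.
; It then checks the player's state and selects the current building when that state is Construction.
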(event `InitBuildingManager`
  ;[1 1 1] Initialize Section
  (bind _asplayer (cast `/Game/Player/Blueprints/Player` (`GameplayStatics.GetPlayerCharacter` 0)))
  (bind _output_get (set `self.PlayerRefBP` _asplayer))
  (bind _returnvalue (`MainWidget.GenerateBuildingWidgets` (`/Game/Player/Blueprints/Player.MainWidgetBP` _output_get) self))
  (set `self.BuildingWidgets` _returnvalue)
  (switch `EPlayerStates` (`RPGSystemCharacter.PlayerStates` (`self.Player`))
    (:`VE_Construction`
      (`self.SelectCurrentBuilding` true))))