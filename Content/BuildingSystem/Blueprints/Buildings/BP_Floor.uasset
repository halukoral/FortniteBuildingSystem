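; BP_Floor is the floor piece of the building system, with its look determined by the resource it is built from.
; Its SetMesh event checks the Resource value and assigns the matching floor static mesh to BuildingMesh: stone, wood, or, for Ice, the metal mesh.
; Any other resource leaves the mesh unchanged, while BeginPlay and the construction script only call their parent versions.
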(event `self.ReceiveBeginPlay`
  (`parent.ReceiveBeginPlay`))

(event `self.SetMesh`
  (params (Resource :type "Resource Class Reference"))
  (if (== Resource "/Script/RPGSystem.Resource_Ice")
    (`StaticMeshComponent.SetStaticMesh` (`self.BuildingMesh`) "/Game/BuildingSystem/Meshes/Metal/SM_FloorMetal.SM_FloorMetal")
    (elif (== Resource "/Script/RPGSystem.Resource_Stone")
      (`StaticMeshComponent.SetStaticMesh` (`self.BuildingMesh`) "/Game/BuildingSystem/Meshes/Stone/SM_FloorStone.SM_FloorStone")
      (elif (== Resource "/Script/RPGSystem.Resource_Wood")
        (`StaticMeshComponent.SetStaticMesh` (`self.BuildingMesh`) "/Game/BuildingSystem/Meshes/Wood/SM_FloorWood.SM_FloorWood")))))

(fn `UserConstructionScript`
  (`parent.UserConstructionScript`))