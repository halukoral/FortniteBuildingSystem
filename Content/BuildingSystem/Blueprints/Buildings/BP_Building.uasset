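; Base-style building actor for the building system that takes damage from the player and is destroyed when its health runs out.
; BeginPlay assigns the build and health bar widget components before running parent logic.
; Damage from a Player lowers the Health stat and passes the impact point to a dynamic material.
; Surviving hits play a timeline that scales the impact normal into the material's Impact parameter for a bounce reaction.
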(event `self.ReceiveBeginPlay`
  (set `self.BuildWidgetComponent` (`self.BPC_BuildWidget`))
  (set `self.HealthBarWidgetComponent` (`self.BPC_HealthBar`))
  (`parent.ReceiveBeginPlay`))

(event `self.ReceiveAnyDamage`
  (params (Damage :type "Float (single-precision)") (DamageType :type "DamageType Object Reference") (InstigatedBy :type "Controller Object Reference") (DamageCauser :type "Actor Object Reference"))
  (bind _dynamicmaterialinstance (`self.DynamicMaterialInstance`))
  (bind _buildingstat (`self.BuildingStat`))
  (bind (_returnvalue_minvalue _returnvalue_currentvalue) (break `StatValues` (`StatManager.GetStat` _buildingstat "VE_Health")))
  (bind _asplayer (cast `/Game/Player/Blueprints/Player` DamageCauser))
  (`MaterialInstanceDynamic.SetVectorParameterValue` _dynamicmaterialinstance "Position" (`KismetMathLibrary.Conv_VectorToLinearColor` (`/Game/Player/Blueprints/Player.ImpactPoint` _asplayer)))
  (`StatManager.ModifyStat` _buildingstat "VE_Health" (`KismetMathLibrary.Round` (* -1 Damage)))
  (if (<= _returnvalue_currentvalue 0)
    (`self.DestroyBuilding`)
    (else
      (bind (_direction _bounce) (`Timeline|Timeline_0` :!via `PlayFromStart`)
        (:`Update`
          (`MaterialInstanceDynamic.SetVectorParameterValue` _dynamicmaterialinstance "Impact" (`KismetMathLibrary.Conv_VectorToLinearColor` (* (`/Game/Player/Blueprints/Player.ImpactNormal` _asplayer) (* _bounce 100.0)))))))))

(fn `UserConstructionScript`)