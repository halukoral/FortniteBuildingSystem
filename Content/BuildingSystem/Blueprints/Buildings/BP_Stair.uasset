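; BP_Stair is the stair piece of the building system, with its look chosen by resource type.
; The SetMesh event swaps the BuildingMesh static mesh to the wood, stone or metal stair for Wood, Stone or Ice, with Ice mapping to the metal mesh.
; Any other resource leaves the mesh unchanged.
; BeginPlay and the construction script only call their parent versions.
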(event `self.ReceiveBeginPlay`
  (`parent.ReceiveBeginPlay`))

(event `self.SetMesh`
  (params (Resource :type "Resource Class Reference"))
  (if (== Resource "/Script/RPGSystem.Resource_Ice")
    (`StaticMeshComponent.SetStaticMesh` (`self.BuildingMesh`) "/Game/BuildingSystem/Meshes/Metal/SM_StairMetal.SM_StairMetal")
    (elif (== Resource "/Script/RPGSystem.Resource_Stone")
      (`StaticMeshComponent.SetStaticMesh` (`self.BuildingMesh`) "/Game/BuildingSystem/Meshes/Stone/SM_StairStone.SM_StairStone")
      (elif (== Resource "/Script/RPGSystem.Resource_Wood")
        (`StaticMeshComponent.SetStaticMesh` (`self.BuildingMesh`) "/Game/BuildingSystem/Meshes/Wood/SM_StairWood.SM_StairWood")))))

(fn `UserConstructionScript`
  (`parent.UserConstructionScript`))