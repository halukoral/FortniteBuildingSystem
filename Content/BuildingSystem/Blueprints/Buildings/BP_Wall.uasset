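; BP_Wall is a wall building piece in the building system whose look depends on its resource.
; Its SetMesh event swaps the BuildingMesh static mesh to a wood, stone or metal wall through a chain of resource checks.
; The Ice resource maps to the metal wall mesh, and any other unmatched resource leaves the mesh unchanged.
; BeginPlay and the construction script only call the parent versions.
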(event `self.ReceiveBeginPlay`
  (`parent.ReceiveBeginPlay`))

(event `self.SetMesh`
  (params (Resource :type "Resource Class Reference"))
  (if (== Resource "/Script/RPGSystem.Resource_Ice")
    (`StaticMeshComponent.SetStaticMesh` (`self.BuildingMesh`) "/Game/BuildingSystem/Meshes/Metal/SM_WallMetal.SM_WallMetal")
    (elif (== Resource "/Script/RPGSystem.Resource_Stone")
      (`StaticMeshComponent.SetStaticMesh` (`self.BuildingMesh`) "/Game/BuildingSystem/Meshes/Stone/SM_WallStone.SM_WallStone")
      (elif (== Resource "/Script/RPGSystem.Resource_Wood")
        (`StaticMeshComponent.SetStaticMesh` (`self.BuildingMesh`) "/Game/BuildingSystem/Meshes/Wood/SM_WallWood.SM_WallWood")))))

(fn `UserConstructionScript`
  (`parent.UserConstructionScript`))