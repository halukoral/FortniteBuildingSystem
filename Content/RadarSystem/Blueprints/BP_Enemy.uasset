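; BP_Enemy is an enemy that patrols to random reachable points around its spawn location and reports itself to a player's radar component.
; Overlaps on RadarSphere add or remove it from that BP_RadarSystem, while OnRadarInit registers it with a radar already in range.
; A looping timer pushes position updates while it moves on radar, with one final update when it stops.
; The construction script applies sphere radii and walk speed.
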(event `self.ReceiveBeginPlay`
  (set `self.StartLocation` (`self.K2_GetActorLocation`))
  (`self.StartPatrolling`))

(event `OnStartMoving`
  (set `self.bCurrentlyMoving` true)
  (if (`self.bOnRadar`)
    (`/Engine/EditorBlueprintResources/StandardMacros.IsValid` (`self.PlayerRadar`)
      (:`Is Valid`
        (`self.UpdateOnRadar`)
        (`self.StartUpdateTimer`)))))

(event `OnStopMoving`
  (set `self.bCurrentlyMoving` false)
  (`KismetSystemLibrary.K2_ClearAndInvalidateTimerHandle` (`self.UpdateRadarTimer`))
  (if (`self.bOnRadar`)
    (`/Engine/EditorBlueprintResources/StandardMacros.IsValid` (`self.PlayerRadar`)
      (:`Is Valid`
        (`self.UpdateOnRadar`)))))

(event `StartPatrolling`
  (`self.OnStartMoving`)
  (`|AIMoveTo` self (`NavigationSystemV1.K2_GetRandomReachablePointInRadius` (`self.StartLocation`) (`self.PatrolRadius`) null null) null
    (:`OnSuccess`
      (`self.OnStopMoving`)
      (`KismetSystemLibrary.Delay` (`KismetMathLibrary.RandomFloatInRange` 1.0 3.0))
      (`self.StartPatrolling`))))

(event `StartUpdateTimer`
  (bind _returnvalue (`KismetSystemLibrary.K2_SetTimerDelegate` (delegate `UpdateOnRadar`) (`self.RadarUpdateInterval`) true))
  (set `self.UpdateRadarTimer` _returnvalue))

(event `UpdateOnRadar`
  (`RadarSystem.OnEnemyMoved` (`self.PlayerRadar`) self))

(event `self.RadarSphere.OnComponentBeginOverlap`
  (params (OverlappedComponent :type "PrimitiveComponent Object Reference") (OtherActor :type "Actor Object Reference") (OtherComp :type "PrimitiveComponent Object Reference") (OtherBodyIndex :type Integer) (bFromSweep :type Boolean) (SweepResult :type "HitResult Structure (by ref)"))
  (bind _returnvalue (`self.GetComponentByClass` OtherActor "/Game/RadarSystem/Blueprints/BP_RadarSystem.BP_RadarSystem_C"))
  (if (not (`self.bOnRadar`))
    (`/Engine/EditorBlueprintResources/StandardMacros.IsValid` _returnvalue
      (:`Is Valid`
        (bind _returnvalue_2 (`RadarSystem.AddEnemy` _returnvalue self))
        (if _returnvalue_2
          (set `self.bOnRadar` true)
          (set `self.PlayerRadar` _returnvalue)
          (if (`self.bCurrentlyMoving`)
            (`self.StartUpdateTimer`)))))))

(event `self.RadarSphere.OnComponentEndOverlap`
  (params (OverlappedComponent :type "PrimitiveComponent Object Reference") (OtherActor :type "Actor Object Reference") (OtherComp :type "PrimitiveComponent Object Reference") (OtherBodyIndex :type Integer))
  (bind _returnvalue (`self.GetComponentByClass` OtherActor "/Game/RadarSystem/Blueprints/BP_RadarSystem.BP_RadarSystem_C"))
  (if (`self.bOnRadar`)
    (`/Engine/EditorBlueprintResources/StandardMacros.IsValid` _returnvalue
      (:`Is Valid`
        (set `self.bOnRadar` false)
        (`KismetSystemLibrary.K2_ClearAndInvalidateTimerHandle` (`self.UpdateRadarTimer`))
        (`RadarSystem.RemoveEnemy` _returnvalue self)
        (set `self.PlayerRadar` null)))))

(event `OnRadarInit`
  (for _array_element (`PrimitiveComponent.GetOverlappingActors` (`self.RadarSphere`) "/Script/Engine.Pawn") :!label _label
    (bind _returnvalue (`self.GetComponentByClass` _array_element "/Game/RadarSystem/Blueprints/BP_RadarSystem.BP_RadarSystem_C"))
    (`/Engine/EditorBlueprintResources/StandardMacros.IsValid` _returnvalue
      (:`Is Valid`
        (bind _returnvalue_2 (`RadarSystem.AddEnemy` _returnvalue self))
        (if _returnvalue_2
          (set `self.bOnRadar` true)
          (set `self.PlayerRadar` _returnvalue)
          (`self.Break`))))))

(event `Break`
  (goto _label :!via `Break`))

(fn `UserConstructionScript`
  (`SphereComponent.SetSphereRadius` (`self.PatrolSphere`) (`self.PatrolRadius`) false)
  (`SphereComponent.SetSphereRadius` (`self.RadarSphere`) (`self.RadarRadius`) false)
  (set `CharacterMovementComponent.MaxWalkSpeed` (`self.MovementSpeed`) (`self.CharacterMovement`)))