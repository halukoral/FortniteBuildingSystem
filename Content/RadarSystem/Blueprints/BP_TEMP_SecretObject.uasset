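; Temporary secret-object actor for the radar system that reveals itself to nearby radar-equipped actors.
; Its Sphere, sized from HighlightRadius in the construction script, detects overlapping actors that have a BP_RadarSystem component.
; On begin and end overlap it notifies that component of entering or leaving secret range and shows or hides its TextRender.
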(event `self.Sphere.OnComponentBeginOverlap`
  (params (OverlappedComponent :type "PrimitiveComponent Object Reference") (OtherActor :type "Actor Object Reference") (OtherComp :type "PrimitiveComponent Object Reference") (OtherBodyIndex :type Integer) (bFromSweep :type Boolean) (SweepResult :type "HitResult Structure (by ref)"))
  (bind _returnvalue (`self.GetComponentByClass` OtherActor "/Game/RadarSystem/Blueprints/BP_RadarSystem.BP_RadarSystem_C"))
  (`/Engine/EditorBlueprintResources/StandardMacros.IsValid` _returnvalue
    (:`Is Valid`
      (`RadarSystem.OnEnterSecretRange` _returnvalue self)
      (`SceneComponent.SetVisibility` (`self.TextRender`) true false))))

(event `self.Sphere.OnComponentEndOverlap`
  (params (OverlappedComponent :type "PrimitiveComponent Object Reference") (OtherActor :type "Actor Object Reference") (OtherComp :type "PrimitiveComponent Object Reference") (OtherBodyIndex :type Integer))
  (bind _returnvalue (`self.GetComponentByClass` OtherActor "/Game/RadarSystem/Blueprints/BP_RadarSystem.BP_RadarSystem_C"))
  (`/Engine/EditorBlueprintResources/StandardMacros.IsValid` _returnvalue
    (:`Is Valid`
      (`RadarSystem.OnLeaveSecretRange` _returnvalue self)
      (`SceneComponent.SetVisibility` (`self.TextRender`) false false))))

(fn `UserConstructionScript`
  (`SphereComponent.SetSphereRadius` (`self.Sphere`) (`self.HighlightRadius`) true))