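; BP_RadarSystem sets up the player's radar widget and fades it in and out.
; InitRadar takes the radar from the player's main widget, adds directions, quests and landmarks, then triggers the visibility callback.
; It then finds every BP_Enemy and notifies each that the radar is initialized.
; Show and hide share one BlendOut animation, played in reverse to show, and store its length as DelayTime.
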(event `self.VisibleAnimation`
  (bind _radarwidgetrefbp (`self.RadarWidgetRefBP`))
  (bind _blendout (`/Game/RadarSystem/Widgets/W_Radar.BlendOut` _radarwidgetrefbp))
  ;[1 1 1] Radar Widget Visibility Blend In Out Animation
  (`UserWidget.PlayAnimation` _radarwidgetrefbp _blendout 0.0 1 "Reverse" 1.0)
  (set `self.DelayTime` (`WidgetAnimation.GetEndTime` _blendout)))

(event `self.HideAnimation`
  (bind _radarwidgetrefbp (`self.RadarWidgetRefBP`))
  (bind _blendout (`/Game/RadarSystem/Widgets/W_Radar.BlendOut` _radarwidgetrefbp))
  ;[1 1 1] Radar Widget Visibility Blend In Out Animation
  (`UserWidget.PlayAnimation` _radarwidgetrefbp _blendout 0.0 1 "Forward" 1.0)
  (set `self.DelayTime` (`WidgetAnimation.GetEndTime` _blendout)))

(event `InitRadar`
  ;[1 1 1] Init Section
  (bind _asplayer (cast `/Game/Player/Blueprints/Player` (`GameplayStatics.GetPlayerCharacter` 0)))
  (bind _radar (`/Game/Widgets/W_Main.Radar` (`/Game/Player/Blueprints/Player.MainWidgetBP` _asplayer)))
  (set `self.RadarWidget` _radar)
  (bind _asw_radar (cast `/Game/RadarSystem/Widgets/W_Radar` _radar))
  (set `self.RadarWidgetRefBP` _asw_radar)
  (`self.AddDirections`)
  (for _array_element (`self.Quests`)
    (`self.AddQuest` _array_element))
  (`self.AddLandmarks`)
  (`self.OnBecomeVisible`)
  (`self.OnRadarInit`))

(event `OnRadarInit`
  (bind _outactors (`GameplayStatics.GetAllActorsOfClass` "/Game/RadarSystem/Blueprints/BP_Enemy.BP_Enemy_C"))
  (for _array_element _outactors
    (`/Game/RadarSystem/Blueprints/BP_Enemy.OnRadarInit` _array_element)))